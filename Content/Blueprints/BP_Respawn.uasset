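; BP_Respawn is a trigger actor that sends the first-person character back to a respawn point on overlap.
; It first calls SetInivsibleFloor on every InvisibleFloor entry and SetPlan on every Plan entry, presumably restoring those level pieces.
; It then moves the character's capsule to the RespawnPoint component's world location without sweep or teleport physics.
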(event `self.ReceiveActorBeginOverlap`
  (params (OtherActor :type "Actor Object Reference"))
  (bind _asbp_first_person_character (cast `/Game/Blueprints/Implemented/BP_FirstPersonCharacter` OtherActor))
  (`|ExecutionSequence`
    (:`then_0`
      (for _array_element (`self.InvisibleFloor`)
        (`/Game/Blueprints/BP_InvisibleFloor.SetInivsibleFloor` _array_element)))
    (:`then_1`
      (for _array_element_2 (`self.Plan`)
        (`/Game/Blueprints/BP_Plan.SetPlan` _array_element_2)))
    (:`then_2`
      (`SceneComponent.K2_SetWorldLocation` (`Character.CapsuleComponent` _asbp_first_person_character) (`SceneComponent.K2_GetComponentLocation` (`self.RespawnPoint`)) false false))))

(fn `UserConstructionScript`)