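; Double-door Blueprint that swings two door meshes open and closed when its Interaction event fires and CanOpen is true.
; A FlipFlop alternates between playing and reversing the RotationAngle timeline.
; The timeline output, scaled by Angle, sets the yaw of the two meshes in opposite directions.
; BeginPlay sets the timeline play rate to the inverse of Duration.
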(event `self.ReceiveBeginPlay`
  (`TimelineComponent.SetPlayRate` (`self.RotationAngle`) (/ 1.0 (`self.Duration`))))

(event `/Game/Blueprints/Implemented/BPI_Interaction.Interaction`
  (if (`self.CanOpen`)
    (`/Engine/EditorBlueprintResources/StandardMacros.FlipFlop`
      (:`A`
        (bind (_direction _angle) (`Timeline|RotationAngle` :!label _label)
          (:`Update`
            (bind _returnvalue (* _angle (`self.Angle`)))
            (`SceneComponent.K2_SetRelativeRotation` (`self.Door_3_StaticMeshComponent0`) (`KismetMathLibrary.MakeRotator` 0.0 0.0 (* _returnvalue -1.0)) false false)
            (`SceneComponent.K2_SetRelativeRotation` (`self.Door_4_StaticMeshComponent0`) (`KismetMathLibrary.MakeRotator` 0.0 0.0 _returnvalue) false false))))
      (:`B`
        (goto _label :!via `Reverse`)))))

(fn `UserConstructionScript`)