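; BP_CodeDoor is a double door that opens when the player types the correct number, which is the count of pumpkins in its Pumpkins array.
; Interaction creates a PlayerTextInput widget, passes it a reference to the door and switches to UI-only input with the mouse cursor shown.
; CheckNb compares the typed number to that count and, on a match, plays the Rotation timeline to swing both doors in opposite directions.
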(event `self.ReceiveBeginPlay`
  (set `self.PumpkinsNb` (`KismetArrayLibrary.Array_Length` (`self.Pumpkins`))))

(event `/Game/Blueprints/Implemented/BPI_Interaction.Interaction`
  (bind _returnvalue (`GameplayStatics.GetPlayerController` 0))
  (bind _returnvalue_2 (`|CreateWidget` "/Game/Blueprints/PlayerTextInput.PlayerTextInput_C"))
  (`|ExecutionSequence`
    (:`then_0`
      (set `/Game/Blueprints/PlayerTextInput.CodeDoor` self _returnvalue_2))
    (:`then_1`
      (`UserWidget.AddToViewport` _returnvalue_2 0)
      (set `PlayerController.bShowMouseCursor` true _returnvalue)
      (`WidgetBlueprintLibrary.SetInputMode_UIOnlyEx` _returnvalue _returnvalue_2))))

(event `CheckNb`
  (if (== (`KismetStringLibrary.Conv_StringToInt` (`KismetTextLibrary.Conv_TextToString` (`/Game/Blueprints/PlayerTextInput.NbText` (stale `/Game/Blueprints/Implemented/BPI_Interaction.Interaction` _returnvalue_2)))) (`self.PumpkinsNb`))
    (`self.OpenDoor`)))

(event `OpenDoor`
  (bind (_direction _newtrack_0) (`Timeline|Rotation`)
    (:`Update`
      (bind _returnvalue (* _newtrack_0 (`self.Angle`)))
      (`SceneComponent.K2_SetRelativeRotation` (`self.Door_2_StaticMeshComponent0`) (`KismetMathLibrary.MakeRotator` 0.0 0.0 _returnvalue) false false)
      (`SceneComponent.K2_SetRelativeRotation` (`self.Door_1_StaticMeshComponent0`) (`KismetMathLibrary.MakeRotator` 0.0 0.0 (* _returnvalue -1.0)) false false))))

(fn `UserConstructionScript`)